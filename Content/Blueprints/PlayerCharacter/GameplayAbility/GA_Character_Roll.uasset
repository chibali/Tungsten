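; Gameplay ability that makes the player character perform a roll in its last movement input direction.
; After a brief delay, it sets motion warping targets for facing and landing point, then plays the roll montage and ends when it finishes.
; The landing point uses a level-scaled distance and a downward trace to find ground, without checking for a hit.
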(event `self.K2_ActivateAbility`
  (`KismetSystemLibrary.Delay` 0.05)
  (`self.ComputeRollDirectionAndDistance`)
  (`AbilityTask_PlayMontageAndWait.CreatePlayMontageAndWaitProxy` "None" "/Game/Blueprints/PlayerCharacter/Animations/AnimationMontages/Equip/AM_Human_RollRT.AM_Human_RollRT"
    (:`OnCompleted`
      _)
    (:`OnBlendOut`
      _)
    (:`OnInterrupted`
      _)
    (:`OnCancelled`
      _))
  (`self.K2_EndAbility`))

(fn `ComputeRollDirectionAndDistance`
  (locals (CachedRollingDirection :type "Vector Structure" :default (0.0 0.0 0.0)))
  (bind _returnvalue (+ (`Actor.K2_GetActorLocation` (`self.GetTungstenCharacterFromActorInfo`)) (* (`local.CachedRollingDirection`) (`TungstenFunctionLibrary.GetScalableFloatValueAtLevel` (`self.RollingDistanceScalableFloat`) (`KismetMathLibrary.Conv_IntToDouble` (`self.GetAbilityLevel`))))))
  (set `local.CachedRollingDirection` (`KismetMathLibrary.Normal` (`Pawn.GetLastMovementInputVector` (`self.GetTungstenCharacterFromActorInfo`))))
  (`|ExecutionSequence`
    (:`then_0`
      (`MotionWarpingComponent.AddOrUpdateWarpTargetFromLocationAndRotation` (`TungstenCharacterBase.MotionWarpingComponent` (`self.GetTungstenCharacterFromActorInfo`)) "RollingDirection" (0.0 0.0 0.0) (`KismetMathLibrary.MakeRotFromX` (`local.CachedRollingDirection`))))
    (:`then_1`
      (bind _outhit (`KismetSystemLibrary.LineTraceSingleForObjects` _returnvalue (+ _returnvalue (* (* (`Actor.GetActorUpVector` (`self.GetTungstenCharacterFromActorInfo`)) -1.0) 500.0)) (`self.Object Types`)))
      (`MotionWarpingComponent.AddOrUpdateWarpTargetFromLocation` (`TungstenCharacterBase.MotionWarpingComponent` (`self.GetTungstenCharacterFromActorInfo`)) "RollingTargetLocation" (`.ImpactPoint` (`GameplayStatics.BreakHitResult` _outhit))))))