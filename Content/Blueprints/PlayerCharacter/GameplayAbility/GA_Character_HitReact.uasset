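; Gameplay ability that plays a directional hit reaction on a Tungsten character when activated by a gameplay event.
; It computes a direction tag from the event instigator and the victim, then picks the front, left, right or back montage.
; While the montage plays, the HitFxSwitch material parameter is switched on.
; Any montage completion, blend-out, interruption or cancellation ends the ability, which switches the effect off.
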(event `self.K2_ActivateAbilityFromEvent`
  (params (EventData :type "GameplayEventData Structure (by ref)"))
  (`|SwitchGameplayTag` (`.ReturnValue` (`TungstenFunctionLibrary.ComputeHitReactDirectionTag` (`.Instigator` (break `GameplayEventData` EventData)) (`self.GetTungstenCharacterFromActorInfo`)))
    (:`Shared.Status.HitReact.Front`
      (set `self.Montage to Play` "/Game/Blueprints/PlayerCharacter/Animations/AnimationMontages/HitReact/AM_Human_HitReact_FrontRT.AM_Human_HitReact_FrontRT"))
    (:`Shared.Status.HitReact.Left`
      (set `self.Montage to Play` "/Game/Blueprints/PlayerCharacter/Animations/AnimationMontages/HitReact/AM_Human_HitReact_LeftRT.AM_Human_HitReact_LeftRT"))
    (:`Shared.Status.HitReact.Right`
      (set `self.Montage to Play` "/Game/Blueprints/PlayerCharacter/Animations/AnimationMontages/HitReact/AM_Human_HitReact_RightRT.AM_Human_HitReact_RightRT"))
    (:`Shared.Status.HitReact.Back`
      (set `self.Montage to Play` "/Game/Blueprints/PlayerCharacter/Animations/AnimationMontages/HitReact/AM_Human_HitReact_BackRT.AM_Human_HitReact_BackRT")))
  (`AbilityTask_PlayMontageAndWait.CreatePlayMontageAndWaitProxy` "None" (`self.Montage to Play`)
    (:`then`
      (`MeshComponent.SetScalarParameterValueOnMaterials` (`self.GetOwningComponentFromActorInfo`) "HitFxSwitch" 1.0))
    (:`OnCompleted`
      (`self.K2_EndAbility` :!label _label))
    (:`OnBlendOut`
      (goto _label))
    (:`OnInterrupted`
      (goto _label))
    (:`OnCancelled`
      (goto _label))))

(event `self.K2_OnEndAbility`
  (params (bWasCancelled :type Boolean))
  (`MeshComponent.SetScalarParameterValueOnMaterials` (`self.GetOwningComponentFromActorInfo`) "HitFxSwitch" 0.0))